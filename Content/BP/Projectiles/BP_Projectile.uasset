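; BP_Projectile is a homing projectile that flies to an assigned target and damages it as an enemy.
; On spawn it rotates once to face the target, then each tick eases toward the target's current location with VInterpTo.
; When the next step lands within a small tolerance, it casts the target to BP_EnemyBase, applies damage and destroys itself.
; It also destroys itself if the target becomes invalid.
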(event `self.ReceiveBeginPlay`
  (`self.LookTarget`))

(event `self.ReceiveTick`
  (params (DeltaSeconds :type "Float (single-precision)"))
  (bind _target (`self.Target`))
  (bind _returnvalue (`self.K2_GetActorLocation` _target))
  (bind _returnvalue_2 (`KismetMathLibrary.VInterpTo` (`self.K2_GetActorLocation`) _returnvalue DeltaSeconds 15.0))
  (`/Engine/EditorBlueprintResources/StandardMacros.IsValid` _target
    (:`Is Valid`
      (if (== _returnvalue_2 _returnvalue :`ErrorTolerance` 10.0)
        (bind _asbp_enemy_base (cast `/Game/BP/Enemies/BP_EnemyBase` (`self.Target`)))
        (`/Game/BP/Enemies/BP_EnemyBase.TakeDamage` _asbp_enemy_base (`self.Damage`))
        (`self.K2_DestroyActor`)
        (else
          (`self.K2_SetActorLocation` _returnvalue_2))))
    (:`Is Not Valid`
      (`self.K2_DestroyActor`))))

(fn `LookTarget`
  (`self.K2_SetActorRotation` (`KismetMathLibrary.FindLookAtRotation` (`self.K2_GetActorLocation`) (`self.K2_GetActorLocation` (`self.Target`)))))

(fn `UserConstructionScript`)