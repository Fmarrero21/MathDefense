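; Player controller for a tower game with a build mode, energy quizzes on towers and a points balance.
; It creates the main game UI on BeginPlay, broadcasts play-mode changes and exits the game on Escape.
; Outside build mode, selecting a tower generates a quiz and shows it in an energy popup at the tower's anchor.
; Quiz results go back to the tower, which is then reselected; TakePoints deducts points when affordable.
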(event `self.ReceiveBeginPlay`
  (`WidgetBlueprintLibrary.SetInputMode_GameAndUIEx` self null "DoNotLock" false)
  (bind _returnvalue (`|CreateWidget` "/Game/UI/WBP_Game_UI.WBP_Game_UI_C" self))
  (bind _output_get (set `self.MainUI` _returnvalue))
  (`UserWidget.AddToPlayerScreen` _output_get 0))

(event `Key|Escape`
  (params (Key :type "Key Structure"))
  (:`Released`
    (`KismetSystemLibrary.ExecuteConsoleCommand` "Exit" null)))

(event `ToggleBuildMode`
  (params (Activate :type Boolean))
  (bind _output_get (set `self.PlayMode` (select `bool` Activate :`false` "NewEnumerator0" :`true` "NewEnumerator1" :!type "/Game/BP/Player/E_PlayerMode Enum")))
  (`self.PlayModeChanged` _output_get))

(event `SelectTower`
  (params (Tower :type "/Game/BP/Towers/BP_Player_Tower Object Reference"))
  (if (`|EnumEquality` (`self.PlayMode`) "NewEnumerator0")
    (bind _output_get (set `self.SelectedTower` Tower))
    (bind _quiz (`/Game/BP/Towers/BP_Player_Tower.GenerateQuiz` _output_get))
    (`/Game/UI/WBP_Game_UI.ShowEnergyPopup` (`self.MainUI`) (`SceneComponent.K2_GetComponentLocation` (`/Game/BP/Towers/BP_Player_Tower.PopupAnchor` _output_get)) _quiz)))

(event `ResolveTowerQuiz`
  (params (Success :type Boolean))
  (bind _selectedtower (`self.SelectedTower`))
  (`/Engine/EditorBlueprintResources/StandardMacros.IsValid` _selectedtower
    (:`Is Valid`
      (`/Game/BP/Towers/BP_Player_Tower.ResolveEnergyQuiz` _selectedtower Success)
      (`self.SelectTower` _selectedtower))))

(fn `TakePoints`
  (params (Quantity :type Integer))
  (returns (Points :type Integer) (ReturnValue :type Boolean))
  (bind _returnvalue (>= (`self.Points`) Quantity))
  (if _returnvalue
    (bind _output_get (set `self.Points` (- (`self.Points`) Quantity))))
  (return _output_get _returnvalue))

(fn `UserConstructionScript`)