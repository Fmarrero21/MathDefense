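; BP_Player_Pawn is a player pawn whose camera spring arm tilts with the mouse wheel.
; Wheel input nudges a clamped 0–1 camera position ratio, which a float curve maps to a target pitch.
; Tick smoothly interpolates the spring arm's relative rotation toward that pitch, keeping roll and yaw unchanged.
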(event `InputAxisKey|MouseWheelAxis`
  (params (AxisValue :type "Float (single-precision)"))
  (bind _output_get (set `self.CameraPositionRatio` (`KismetMathLibrary.FClamp` (+ (* AxisValue 0.05) (`self.CameraPositionRatio`)))))
  (set `self.TargetRotation` (`CurveFloat.GetFloatValue` (`self.RotationCurve`) _output_get)))

(event `self.ReceiveTick`
  (params (DeltaSeconds :type "Float (single-precision)"))
  (bind _relativerotation (`SceneComponent.RelativeRotation` (`self.SpringArm`)))
  (`SceneComponent.K2_SetRelativeRotation` (`self.SpringArm`) (`KismetMathLibrary.RInterpTo` _relativerotation (`KismetMathLibrary.MakeRotator` (.roll _relativerotation) (`self.TargetRotation`) (.yaw _relativerotation)) DeltaSeconds 5.0) false false))

(fn `UserConstructionScript`)