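; BP_EnemySpawner periodically spawns BP_EnemyBase enemies around its own location.
; On BeginPlay it caches every BP_Lane_Choice actor as Choices, currently unordered, then starts a looping timer at SpawnTime.
; Each tick of the timer picks a random navigable point within a fixed radius and spawns an enemy there, adjusting for collisions and passing it the lane choices.
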(event `GetLaneChoices`
  ;[1 1 1] For now there is only one choice but in the future we need to get all the choices on the mapo and order them by proximity
  (bind _outactors (`GameplayStatics.GetAllActorsOfClass` "/Game/BP/Lane/BP_Lane_Choice.BP_Lane_Choice_C"))
  (set `self.Choices` _outactors))

(event `self.ReceiveBeginPlay`
  (`self.GetLaneChoices`)
  (bind _returnvalue (`KismetSystemLibrary.K2_SetTimerDelegate` (delegate `SpawnEnemy`) (`self.SpawnTime`) true))
  (set `self.Timer` _returnvalue))

(event `SpawnEnemy`
  (bind (_randomlocation _returnvalue) (`NavigationSystemV1.K2_GetRandomLocationInNavigableRadius` (`self.K2_GetActorLocation`) 300.0 null null))
  (if _returnvalue
    (`|SpawnActorFromClass` "/Game/BP/Enemies/BP_EnemyBase.BP_EnemyBase_C" (`KismetMathLibrary.MakeTransform` _randomlocation) "AdjustIfPossibleButDontSpawnIfColliding" "MultiplyWithRoot" null (`self.Choices`) null)))

(fn `UserConstructionScript`)