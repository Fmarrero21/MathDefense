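; Base enemy pawn that walks a branching path to the core tower, damages it on arrival and destroys itself.
; AI MoveTo visits a random point from each successive Choices entry, then targets the CoreTower held by BP_MainGameState.
; Taking damage lowers health and plays a timeline driving mesh custom primitive data.
; At zero health it awards points through BP_PlayerController, stops moving and sets a Dead flag without destroying itself.
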(event `self.ReceiveBeginPlay`
  (set `CharacterMovementComponent.MaxWalkSpeed` (`self.Speed`) (`self.CharacterMovement`))
  (`self.MoveToNextPoint`))

(event `MoveToNextPoint`
  (if (== (`self.ChoiceIdx`) (`KismetArrayLibrary.Array_Length` (`self.Choices`)))
    (bind _asbp_main_game_state (cast `/Game/BP/GameMode/BP_MainGameState` (`GameplayStatics.GetGameState`)))
    (set `self.NextDestination` (`self.K2_GetActorLocation` (`/Game/BP/GameMode/BP_MainGameState.CoreTower` _asbp_main_game_state)))
    (else
      (bind _choicelocation (`/Game/BP/Lane/BP_Lane_Choice.GetRandomChoice` (`|GetArrayItem` (`self.Choices`) (`self.ChoiceIdx`))))
      (set `self.NextDestination` _choicelocation)))
  (`|AIMoveTo` self (`self.NextDestination`) null 80.0 true
    (:`OnSuccess`
      (bind _result (`/Engine/EditorBlueprintResources/StandardMacros.IncrementInt` (`self.ChoiceIdx`))
        (:`  `
          (if (> _result (`KismetArrayLibrary.Array_Length` (`self.Choices`)))
            (`self.OnTargetReach`)
            (else
              (`self.MoveToNextPoint`))))))))

(event `TakeDamage`
  (params (Damage :type "Float (double-precision)"))
  (bind _output_get (set `self.ActualHealth` (`KismetMathLibrary.FMax` (- (`self.ActualHealth`) Damage))))
  (`|ExecutionSequence`
    (:`then_0`
      (bind (_direction _damagefx) (`Timeline|DamageFX` :!via `PlayFromStart`)
        (:`Update`
          (`PrimitiveComponent.SetCustomPrimitiveDataFloat` (`self.Mesh`) 0 _damagefx))))
    (:`then_1`
      (if (== _output_get 0.0)
        (`self.Die`)))))

(event `Die`
  (bind _asbp_player_controller (cast `/Game/BP/Player/BP_PlayerController` (`GameplayStatics.GetPlayerController` 0)))
  (`/Game/BP/Player/BP_PlayerController.AddPoints` _asbp_player_controller (`self.PointsReward`))
  (`Controller.StopMovement` (`self.GetController`))
  (set `self.Dead` true))

(event `OnTargetReach`
  (bind _asbp_main_game_state (cast `/Game/BP/GameMode/BP_MainGameState` (`GameplayStatics.GetGameState`)))
  (`/Game/BP/Towers/BP_Tower_Base.TakeDamage` (`/Game/BP/GameMode/BP_MainGameState.CoreTower` _asbp_main_game_state) (`self.Damage`))
  (`self.K2_DestroyActor`))

(fn `UserConstructionScript`)