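; BP_Player_Tower is a defense tower that fires projectiles at enemies and spends energy per shot, shown on an energy bar widget.
; A radius sphere tracks enemies in range, and a looping timer fires at the first listed one when energy suffices.
; Clicking selects the tower through the player controller.
; It generates three-option addition quizzes, and quiz results add or drain energy.
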(event `self.ReceiveBeginPlay`
  (`KismetSystemLibrary.K2_SetTimerDelegate` (delegate `ExecuteAction`) (`self.ActionInverval`) true)
  (bind _aswbp_tower_energy (cast `/Game/UI/LevelUI/WBP_Tower_Energy` (`WidgetComponent.GetWidget` (`self.EnergyBar`))))
  (`/Game/UI/LevelUI/WBP_Tower_Energy.SetTower` _aswbp_tower_energy self))

(event `ExecuteAction`
  (bind _energycost (`self.EnergyCost`))
  (if (> (`KismetArrayLibrary.Array_Length` (`self.EnemyList`)) 0)
    ;[0 0 0] Take The energy from the tower
    (bind (_maxenergy _currentenergy) (`self.GetEnergyInfo`))
    (if (>= _currentenergy _energycost)
      (`self.TakeEnergy` _energycost)
      (`|SpawnActorFromClass` "/Game/BP/Projectiles/BP_Projectile.BP_Projectile_C" (`KismetMathLibrary.MakeTransform` (`SceneComponent.K2_GetComponentLocation` (`self.Projectile`))) "AlwaysSpawn" "MultiplyWithRoot" null (`|GetArrayItem` (`self.EnemyList`)) (`self.Damage`) null))))

(event `self.RadiusSphere.OnComponentBeginOverlap`
  (params (OverlappedComponent :type "PrimitiveComponent Object Reference") (OtherActor :type "Actor Object Reference") (OtherComp :type "PrimitiveComponent Object Reference") (OtherBodyIndex :type Integer) (bFromSweep :type Boolean) (SweepResult :type "HitResult Structure (by ref)"))
  (bind _asbp_enemy_base (cast `/Game/BP/Enemies/BP_EnemyBase` OtherActor))
  (`KismetArrayLibrary.Array_AddUnique` (`self.EnemyList`) _asbp_enemy_base))

(event `self.RadiusSphere.OnComponentEndOverlap`
  (params (OverlappedComponent :type "PrimitiveComponent Object Reference") (OtherActor :type "Actor Object Reference") (OtherComp :type "PrimitiveComponent Object Reference") (OtherBodyIndex :type Integer))
  (bind _asbp_enemy_base (cast `/Game/BP/Enemies/BP_EnemyBase` OtherActor))
  (`KismetArrayLibrary.Array_RemoveItem` (`self.EnemyList`) _asbp_enemy_base))

(event `self.Box.OnClicked`
  (params (TouchedComponent :type "PrimitiveComponent Object Reference") (ButtonPressed :type "Key Structure"))
  (bind _asbp_player_controller (cast `/Game/BP/Player/BP_PlayerController` (`GameplayStatics.GetPlayerController` 0)))
  (`/Game/BP/Player/BP_PlayerController.SelectTower` _asbp_player_controller self))

(event `ResolveEnergyQuiz`
  (params (Success :type Boolean))
  (bind _energyrecovery (`self.EnergyRecovery`))
  (if Success
    (`self.AddEnergy` _energyrecovery)
    (else
      (`self.TakeEnergy` _energyrecovery))))

(fn `GenerateQuiz`
  (returns (Quiz :type "/Game/BP/EnergySolver/FQuiz Structure"))
  (locals (X :type Integer :default 0) (Y :type Integer :default 0) (Options :type "Array of Integer") (CurrentOption :type Integer :default 0))
  (bind _options (`local.Options`))
  (bind _output_get (set `local.X` (`KismetMathLibrary.RandomIntegerInRange` 1 9)))
  (bind _output_get_2 (set `local.Y` (`KismetMathLibrary.RandomIntegerInRange` 1 9)))
  (bind _returnvalue (+ _output_get _output_get_2))
  (`KismetArrayLibrary.Array_Add` _options _returnvalue)
  (for _ (range 1 3)
    (bind _returnvalue_2 (+ (`KismetMathLibrary.RandomIntegerInRange` -5 5) _returnvalue))
    (bind _output_get_3 (set `local.CurrentOption` _returnvalue_2))
    (while (or (`KismetArrayLibrary.Array_Contains` (`local.Options`) _output_get_3) (<= _output_get_3 1))
      (set `local.CurrentOption` _returnvalue_2))
    (`KismetArrayLibrary.Array_Add` (`local.Options`) (`local.CurrentOption`)))
  (`KismetArrayLibrary.Array_Shuffle` _options)
  (return (make `/Game/BP/EnergySolver/FQuiz` (`KismetStringLibrary.Concat_StrStr` (`KismetStringLibrary.Conv_IntToString` (`local.X`)) "+" (`KismetStringLibrary.Conv_IntToString` (`local.Y`)) "= ?") (`local.Options`) _returnvalue)))

(fn `UserConstructionScript`
  (`SphereComponent.SetSphereRadius` (`self.RadiusSphere`) (`self.Radius`) false))