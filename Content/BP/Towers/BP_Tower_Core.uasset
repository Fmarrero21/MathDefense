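; BP_Tower_Core is the core tower, whose destruction ends the game.
; On BeginPlay it registers itself with BP_MainGameState as the core tower and binds itself to the WBP_Tower_Health widget held by its HealthStat component.
; Its DestroyTower override runs the parent logic, then calls GameOver on the game state.
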(event `self.ReceiveBeginPlay`
  (bind _asbp_main_game_state (cast `/Game/BP/GameMode/BP_MainGameState` (`GameplayStatics.GetGameState`)))
  (`/Game/BP/GameMode/BP_MainGameState.SetCoreTower` _asbp_main_game_state self)
  (bind _aswbp_tower_health (cast `/Game/UI/LevelUI/WBP_Tower_Health` (`WidgetComponent.GetWidget` (`self.HealthStat`))))
  (`/Game/UI/LevelUI/WBP_Tower_Health.SetTower` _aswbp_tower_health self))

(event `self.DestroyTower`
  (`parent.DestroyTower`)
  (bind _asbp_main_game_state (cast `/Game/BP/GameMode/BP_MainGameState` (`GameplayStatics.GetGameState`)))
  (`/Game/BP/GameMode/BP_MainGameState.GameOver` _asbp_main_game_state))

(fn `UserConstructionScript`)