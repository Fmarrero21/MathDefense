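; Base tower Blueprint that tracks health and energy for towers.
; Damage and energy-drain events clamp values at zero, while energy gain caps at the maximum, and each change fires a health or energy change call.
; Getter functions return max, current and ratio for both stats.
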(event `TakeDamage`
  (params (Damage :type "Float (double-precision)"))
  (set `self.CurrentHealth` (`KismetMathLibrary.FMax` (- (`self.CurrentHealth`) Damage)))
  (`self.OnHealthChange`))

(event `TakeEnergy`
  (params (Energy :type "Float (double-precision)"))
  (set `self.CurrentEnergy` (`KismetMathLibrary.FMax` (- (`self.CurrentEnergy`) Energy)))
  (`self.OnEnergyChange`))

(event `AddEnergy`
  (params (Energy :type "Float (double-precision)"))
  (set `self.CurrentEnergy` (`KismetMathLibrary.FMin` (+ (`self.CurrentEnergy`) Energy) (`self.MaxEnergy`)))
  (`self.OnEnergyChange`))

(fn `GetEnergyInfo`
  (returns (MaxEnergy :type "Float (double-precision)") (CurrentEnergy :type "Float (double-precision)") (Ratio :type "Float (double-precision)"))
  (bind _maxenergy (`self.MaxEnergy`))
  (bind _currentenergy (`self.CurrentEnergy`))
  (return _maxenergy _currentenergy (/ _currentenergy _maxenergy)))

(fn `GetHealthInfo`
  (returns (MaxHealth :type "Float (double-precision)") (CurrentHealth :type "Float (double-precision)") (Ratio :type "Float (double-precision)"))
  (bind _maxhealth (`self.MaxHealth`))
  (bind _currenthealth (`self.CurrentHealth`))
  (return _maxhealth _currenthealth (/ _currenthealth _maxhealth)))

(fn `UserConstructionScript`)