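; Tower build slot actor that lets the player place a tower at a fixed spot in the level.
; It listens to the player controller's play mode changes, showing its clickable display only in Building mode while still empty.
; A click checks mode, points and occupancy, then deducts a temporary fixed cost and spawns BP_Player_Tower at TowerOrigin.
; The slot then stores the tower, marks itself built and hides.
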(event `self.ReceiveBeginPlay`
  (bind _asbp_player_controller (cast `/Game/BP/Player/BP_PlayerController` (`GameplayStatics.GetPlayerController` 0)))
  (add `/Game/BP/Player/BP_PlayerController.PlayModeChanged` _asbp_player_controller (delegate `PlayModeChanged`))
  (`self.PlayModeChanged` (`/Game/BP/Player/BP_PlayerController.PlayMode` _asbp_player_controller)))

(event `PlayModeChanged`
  (params (PlayMode :type "/Game/BP/Player/E_PlayerMode Enum" :default "NewEnumerator0"))
  (bind _slotdisplay (`self.SlotDisplay`))
  ;[0 0 0] When player mode change we show or hide the slots for building towers
  (switch `/Game/BP/Player/E_PlayerMode` PlayMode
    (:`NewEnumerator0`
      (`SceneComponent.SetVisibility` _slotdisplay false true))
    (:`NewEnumerator1`
      (if (not (`self.Builded`))
        (`SceneComponent.SetVisibility` _slotdisplay true true)))))

(event `self.SlotDisplay.OnClicked`
  (params (TouchedComponent :type "PrimitiveComponent Object Reference") (ButtonPressed :type "Key Structure"))
  (if (`self.CanBuild?` 100)
    ;[1 1 1] Take Points from player and build the tower
    (bind _asbp_player_controller (cast `/Game/BP/Player/BP_PlayerController` (`GameplayStatics.GetPlayerController` 0)))
    (`/Game/BP/Player/BP_PlayerController.TakePoints` _asbp_player_controller 100)
    (bind _returnvalue (`|SpawnActorFromClass` "/Game/BP/Towers/BP_Player_Tower.BP_Player_Tower_C" (`KismetMathLibrary.MakeTransform` (`SceneComponent.K2_GetComponentLocation` (`self.TowerOrigin`))) "Undefined" "MultiplyWithRoot" null null))
    (set `self.TowerRef` _returnvalue)
    (set `self.Builded` true)
    (`SceneComponent.SetVisibility` (`self.SlotDisplay`) false true)))

(fn `CanBuild?`
  (params (Cost :type Integer :default 100))
  (returns (ReturnValue :type Boolean))
  (bind _asbp_player_controller (cast `/Game/BP/Player/BP_PlayerController` (`GameplayStatics.GetPlayerController` 0))
    (:`then`
      _)
    (:`CastFailed`
      _))
  (return (and (not (`self.Builded`)) (>= (`/Game/BP/Player/BP_PlayerController.Points` _asbp_player_controller) Cost) (`|EnumEquality` (`/Game/BP/Player/BP_PlayerController.PlayMode` _asbp_player_controller) "NewEnumerator1"))))

(fn `UserConstructionScript`)